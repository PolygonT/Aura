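; Enemy character Blueprint that supplies visual feedback and warp targeting through events.
; A timeline drives the Dissolve scalar parameter on each passed-in material instance to animate a dissolve effect.
; The critical hit event plays an animation on the health bar's progress bar widget.
; Facing updates set the FacingTarget location in Motion Warping, so warped animations can orient toward a target.
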(event `self.StartDissolveTimeline`
  (params (MaterialInstance :type "Array of MaterialInstanceDynamic Object Reference (by ref)"))
  (bind (_direction _dissolvetrack) (`Timeline|DissolveTimeline`)
    (:`Update`
      (for _array_element MaterialInstance
        (`MaterialInstanceDynamic.SetScalarParameterValue` _array_element "Dissolve" _dissolvetrack)))))

(event `self.CriticalHitEvent`
  (bind _aswbp_progress_bar (cast `/Game/Blueprints/UI/ProgressBar/WBP_ProgressBar` (`WidgetComponent.GetUserWidgetObject` (`self.HealthBar`))))
  (`/Game/Blueprints/UI/ProgressBar/WBP_ProgressBar.PlayCriticalHitAnim` _aswbp_progress_bar))

(event `self.ReceiveTick`
  (params (DeltaSeconds :type "Float (single-precision)")))

(event `CombatInterface.UpdateFacingTarget`
  (params (Target :type "Vector Structure (by ref)"))
  (`MotionWarpingComponent.AddOrUpdateWarpTargetFromLocation` (`self.MotionWarping`) "FacingTarget" Target))

(fn `UserConstructionScript`)