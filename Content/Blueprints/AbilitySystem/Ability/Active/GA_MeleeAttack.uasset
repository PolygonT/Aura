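; Gameplay ability for an enemy melee attack that turns the enemy toward its combat target and damages players caught by the hit.
; It plays a random tagged attack montage and waits for the gameplay event matching that montage's tag.
; On the event it damages live players in a small sphere at the tag's combat socket, fires a melee impact gameplay cue if anyone was hit, then ends the ability.
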(event `self.K2_ActivateAbility`
  (bind _as_enemy (`self.As Enemy`))
  (`|ExecutionSequence`
    (:`then_0`
      ; 1. Store Avatar Actor as Enemy and call Update Facing Target Event
      (bind _asenemy (cast `Enemy` (`self.GetAvatarActorFromActorInfo`)))
      (bind _output_get (set `self.As Enemy` _asenemy))
      (`CombatInterface.UpdateFacingTarget` _output_get (`Actor.K2_GetActorLocation` (`EnemyInterface.GetCombatTarget` _output_get)))
      (set `self.HasHitTarget` false))
    (:`then_1`
      ; 2. Play Attack Montage And Cause Damge
      (bind _returnvalue (`CombatInterface.GetAttackMontages` (`self.As Enemy`)))
      (bind _returnvalue_2 (`DefaultAbilitySystemLibrary.GetRandomElementOfTagArr` _returnvalue))
      (bind _output_get_2 (set `self.TaggedMontage` _returnvalue_2))
      (bind (_montage _montagetag) (break `TaggedMontage` _output_get_2))
      (set `self.Montage Tag` _montagetag)
      (`AbilityTask_PlayMontageAndWait.CreatePlayMontageAndWaitProxy` "None" _montage
        (:`then`
          (`AbilityTask_WaitGameplayEvent.WaitGameplayEvent` (`self.Montage Tag`) null
            (:`EventReceived`
              (bind _returnvalue_3 (`CombatInterface.GetCombatSocketLocation` (`self.As Enemy`) (`self.Montage Tag`)))
              (bind _outoverlappingactors (`DefaultAbilitySystemLibrary.GetLivePlayersWithinRadius` _as_enemy (`|MakeArray` _as_enemy :!type "Actor Object Reference") 45.0 _returnvalue_3))
              (for _array_element _outoverlappingactors
                (`self.CauseDamage` _array_element)
                (set `self.HasHitTarget` true))
              (if (`self.HasHitTarget`)
                (`self.K2_ExecuteGameplayCueWithParams` (struct :`TagName` "GameplayCue.MeleeImpact") (`AbilitySystemBlueprintLibrary.MakeGameplayCueParameters` 0.0 0.0 (struct) (struct) (struct) (struct) (struct) _returnvalue_3 (0.0 0.0 0.0) null null (`self.As Enemy`))))
              (`self.K2_EndAbility`))))))))