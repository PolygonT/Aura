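; Gameplay ability for a channeled lightning shock that lasts while input is held and its cost can be paid.
; A looping timer commits the cost from activation and ends the ability when that fails.
; The cast montage's gameplay event spawns BP_LightningArea at the combat socket, enters the shock loop state and awaits input release.
; Both endings call OnEndAbility, which exits combat state, commits cooldown, clears the timer and destroys the area.
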(event `CostEvent`
  ; Commit Cost
  (bind _returnvalue (`self.K2_CommitAbilityCost` false))
  (if (not _returnvalue)
    (`self.OnEndAbility`)
    (`self.K2_EndAbility`)))

(event `self.K2_ActivateAbility`
  (bind _returnvalue (`self.GetAvatarActorFromActorInfo`))
  (bind _returnvalue_2 (`BlueprintGameplayTagLibrary.MakeLiteralGameplayTag` (struct :`TagName` "Montage.Attack.Weapon")))
  (bind _as_pawn (`self.As Pawn`))
  (`|ExecutionSequence`
    (:`then_0`
      ; Commit Cost
      (bind _returnvalue_3 (`KismetSystemLibrary.K2_SetTimerDelegate` (delegate `CostEvent`) 0.1 true))
      (set `self.CostTimer` _returnvalue_3)
      (bind _aspawn (cast `Pawn` (`self.GetAvatarActorFromActorInfo`)))
      (set `self.As Pawn` _aspawn))
    (:`then_1`
      ; Play Montage and Spawn Actor
      (`AbilityTask_PlayMontageAndWait.CreatePlayMontageAndWaitProxy` "None" "/Game/Assets/Characters/Aura/Animations/Abilities/AM_Cast_Shock.AM_Cast_Shock"
        (:`then`
          (`AbilityTask_WaitGameplayEvent.WaitGameplayEvent` _returnvalue_2 null
            (:`EventReceived`
              (bind _returnvalue_4 (message `CombatInterface.GetCombatSocketLocation` _returnvalue _returnvalue_2))
              (bind _returnvalue_5 (`|SpawnActorFromClass` "/Game/Blueprints/Actor/Area/BP_LightningArea.BP_LightningArea_C" (`KismetMathLibrary.MakeTransform` _returnvalue_4 (`Actor.K2_GetActorRotation` _returnvalue)) "Undefined" "MultiplyWithRoot" _as_pawn _as_pawn))
              (set `self.EffectActor` _returnvalue_5)
              ; Change Character State
              (message `CombatInterface.StartCombatState` (`self.GetAvatarActorFromActorInfo`) "CastShockLoop")
              (`AbilityTask_WaitInputRelease.WaitInputRelease` true
                (:`OnRelease`
                  ; Commit Cooldown And Clear CostTimer
                  (`self.OnEndAbility`)
                  (`self.K2_EndAbility`))))))))))

(fn `OnEndAbility`
  (message `CombatInterface.EndCombatState` (`self.GetAvatarActorFromActorInfo`))
  (`self.K2_CommitAbilityCooldown` false)
  (`KismetSystemLibrary.K2_ClearAndInvalidateTimerHandle` (`self.CostTimer`))
  (`Actor.K2_DestroyActor` (`self.EffectActor`)))