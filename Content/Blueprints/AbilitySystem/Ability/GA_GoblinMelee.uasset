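; Goblin spear melee gameplay ability that damages live players near the enemy's combat socket.
; On activation, it turns the avatar Enemy toward its combat target and plays the spear attack montage.
; A melee montage gameplay event triggers a small radius query at the socket, applies damage to each player found, then ends the ability.
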(event `self.K2_ActivateAbility`
  (bind _asenemy (cast `Enemy` (`self.GetAvatarActorFromActorInfo`)))
  (bind _output_get (set `self.As Enemy` _asenemy))
  (`CombatInterface.UpdateFacingTarget` _output_get (`Actor.K2_GetActorLocation` (`EnemyInterface.GetCombatTarget` _output_get)))
  (`AbilityTask_PlayMontageAndWait.CreatePlayMontageAndWaitProxy` "None" "/Game/Assets/Enemies/Goblin/Animations/Spear/AM_GoblinSpear_Attack.AM_GoblinSpear_Attack"
    (:`then`
      (`AbilityTask_WaitGameplayEvent.WaitGameplayEvent` (struct :`TagName` "Event.Montage.Attack.Melee") null
        (:`EventReceived`
          (bind _returnvalue (`CombatInterface.GetCombatSocketLocation` (`self.As Enemy`)))
          (bind _outoverlappingactors (`DefaultAbilitySystemLibrary.GetLivePlayersWithinRadius` (`self.As Enemy`) (`|MakeArray` null :!type "Actor Object Reference") 15.0 _returnvalue))
          (for _array_element _outoverlappingactors
            (`self.CauseDamage` _array_element))
          (`self.K2_EndAbility`))))))