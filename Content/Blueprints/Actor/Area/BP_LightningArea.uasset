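; BP_LightningArea is a lightning area actor with an adjustable length, pairing a capsule collision component with a Niagara beam.
; SetAreaLength stores the length and fires OnAreaLengthChanged, which sets the capsule half height to half the length and shifts it forward on X by that amount.
; The same event writes the length to the Beam End X parameter, keeping visual and collision in step.
; No overlap or damage logic is implemented here.
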(event `Event OnAreaLengthChanged`
  (bind _collisioncomponent (`self.CollisionComponent`))
  (`CapsuleComponent.SetCapsuleHalfHeight` (`self.CollisionComponent`) (`KismetMathLibrary.SafeDivide` (`self.AreaLength`) 2.0) true)
  (`SceneComponent.K2_SetRelativeLocation` _collisioncomponent (`KismetMathLibrary.MakeVector` (`CapsuleComponent.CapsuleHalfHeight` _collisioncomponent)) false false)
  (`NiagaraComponent.SetVariableVec3` (`self.Niagara`) "Beam End" (`KismetMathLibrary.MakeVector` (`self.AreaLength`))))

(event `self.ReceiveBeginPlay`)

(fn `SetAreaLength`
  (params (AreaLength :type "Float (double-precision)"))
  (set `self.AreaLength` AreaLength)
  (`self.Event OnAreaLengthChanged`))

(fn `UserConstructionScript`)