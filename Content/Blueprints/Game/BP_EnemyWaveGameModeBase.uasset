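; Game mode Blueprint that advances enemy waves and announces each one on screen.
; BeginPlay binds to the enemy count change event and calls NextWave once the count drops to zero or below.
; WaveStart shows a wave number message and a countdown widget near the top of the screen.
; A Sequence runs both widgets side by side, each removed after its own Delay, with the countdown's tied to StartTime.
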(event `self.ReceiveBeginPlay`
  (add `DefaultGameModeBase.OnEnemyCountChange` (delegate `OnEnemyCountChange_Event`)))

(event `OnEnemyCountChange_Event`
  (params (EnemyCount :type Integer))
  (if (<= EnemyCount 0)
    (`self.NextWave`)))

(event `self.WaveStart`
  (params (Message :type "Text (by ref)") (StartTime :type "Float (single-precision)") (OutWaveCount :type Integer))
  (bind _messagewidget (`self.MessageWidget`))
  (bind _timerwidget (`self.TImerWidget`))
  (`|ExecutionSequence`
    (:`then_0`
      ; 消息组件
      (bind _returnvalue (`|CreateWidget` "/Game/Blueprints/UI/Overlay/SubWidget/WBP_Common_Message.WBP_Common_Message_C" (`GameplayStatics.GetPlayerController` 0)))
      (bind _output_get (set `self.MessageWidget` _returnvalue))
      (`/Game/Blueprints/UI/Overlay/SubWidget/WBP_Common_Message.SetText` _output_get (`|FormatText` "Wave {Wave}: {Message}" OutWaveCount Message))
      (`UserWidget.SetAnchorsInViewport` (`self.MessageWidget`) (make `Anchors` (0.5 0.2) (0.5 0.2)))
      (`UserWidget.SetAlignmentInViewport` _messagewidget (0.5 0.5))
      (`UserWidget.AddToViewport` _messagewidget 0)
      (`KismetSystemLibrary.Delay` 2.0)
      (`Widget.RemoveFromParent` (`self.MessageWidget`)))
    (:`then_1`
      ; 计时组件
      (bind _returnvalue_2 (`|CreateWidget` "/Game/Blueprints/UI/Overlay/SubWidget/WBP_Countdown.WBP_Countdown_C" (`GameplayStatics.GetPlayerController` 0)))
      (bind _output_get_2 (set `self.TImerWidget` _returnvalue_2))
      (`/Game/Blueprints/UI/Overlay/SubWidget/WBP_Countdown.StartTimer` _output_get_2 StartTime)
      (`UserWidget.SetAnchorsInViewport` (`self.TImerWidget`) (make `Anchors` (0.5 0.17) (0.5 0.17)))
      (`UserWidget.SetAlignmentInViewport` _timerwidget (0.5 0.5))
      (`UserWidget.AddToViewport` _timerwidget 0)
      (`KismetSystemLibrary.Delay` (+ StartTime 0.2))
      (`Widget.RemoveFromParent` (`self.TImerWidget`)))))

(fn `UserConstructionScript`)